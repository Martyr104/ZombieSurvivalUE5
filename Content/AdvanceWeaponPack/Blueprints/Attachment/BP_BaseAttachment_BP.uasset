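; Base pickup actor for weapon attachments that the first-person character collects into its attachment inventory.
; A radius overlap tracks range; while in range and the player's hit component is its Box, Tick shows the pickup HUD with the attachment's name and image.
; The player's pickup event adds the actor's class to the inventory and destroys it under those same conditions.
; The HUD collapses whenever the mouse cursor is shown.
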(event OnComponentBeginOverlap(PickUpRadius)
  (params (OverlappedComponent :type Primitive%20Component%20Object%20Reference) (OtherActor :type Actor%20Object%20Reference) (OtherComp :type Primitive%20Component%20Object%20Reference) (OtherBodyIndex :type Integer) (bFromSweep :type Boolean) (SweepResult :type Hit%20Result%20Structure%20%28by%20ref%29))
  ;[1 1 1] Is Player in range?
  (Utilities|Casting|CastToBP_FirstPersonCharacter OtherActor)
  (Variables|Default|SetIsInRange? true))

(event OnComponentEndOverlap(PickUpRadius)
  (params (OverlappedComponent :type Primitive%20Component%20Object%20Reference) (OtherActor :type Actor%20Object%20Reference) (OtherComp :type Primitive%20Component%20Object%20Reference) (OtherBodyIndex :type Integer))
  (bind _player (Variables|Default|GetPlayer))
  (bind _pickuphud (Variables|/Game/AdvanceWeaponPack/FirstPersonContent/Blueprints/BP_FirstPersonCharacter.BP_FirstPersonCharacter_C|GetPickUpHud _player))
  ;[1 1 1] Is Player in range?
  (Utilities|Casting|CastToBP_FirstPersonCharacter OtherActor)
  (Variables|Default|SetIsInRange? false)
  (Utilities|IsValid _player
    (:Is%20Valid
      (Variables|/Game/AdvanceWeaponPack/Widget/PickUpHUD.PickUpHUD_C|SetIsInRange? _pickuphud false)
      (Widget|SetVisibility _pickuphud "Hidden"))))

(event Custom|PickUp_Event
  (bind _player (Variables|Default|GetPlayer))
  ;[1 1 1] PickUp
  (if (and (== (Variables|/Game/AdvanceWeaponPack/FirstPersonContent/Blueprints/BP_FirstPersonCharacter.BP_FirstPersonCharacter_C|GetHitComponent _player) (Variables|Default|GetBox)) (Variables|Default|GetIsInRange?))
    (Default|AddItem (Variables|/Game/AdvanceWeaponPack/FirstPersonContent/Blueprints/BP_FirstPersonCharacter.BP_FirstPersonCharacter_C|GetBp_Inventory_Attachment _player) (Utilities|GetClass self))
    (Actor|DestroyActor)))

(event EventBeginPlay
  ;[1 1 1] PickUp
  (bind _asbp_first_person_character (Utilities|Casting|CastToBP_FirstPersonCharacter (Game|GetPlayerCharacter 0)))
  (bind _output_get (Variables|Default|SetPlayer _asbp_first_person_character))
  (EventDispatchers|BindEventtoPickUp _output_get (delegate Custom|PickUp_Event)))

(event EventTick
  (params (DeltaSeconds :type Float%20%28single-precision%29))
  (bind _inventorystruct (Variables|Default|GetInventoryStruct))
  (bind _player (Variables|Default|GetPlayer))
  (bind _player_2 (Variables|Default|GetPlayer))
  (bind (_itemmesh _itemimage _attachmenttype) (Utilities|Struct|BreakInventory_Struct _inventorystruct))
  (bind _pickuphud (Variables|/Game/AdvanceWeaponPack/FirstPersonContent/Blueprints/BP_FirstPersonCharacter.BP_FirstPersonCharacter_C|GetPickUpHud _player))
  (bind _pickuphud_2 (Variables|/Game/AdvanceWeaponPack/FirstPersonContent/Blueprints/BP_FirstPersonCharacter.BP_FirstPersonCharacter_C|GetPickUpHud _player_2))
  (bind _attachmentimage (Variables|/Game/AdvanceWeaponPack/Widget/PickUpHUD.PickUpHUD_C|GetAttachmentImage _pickuphud_2))
  ;[1 1 1] Set Name and Image to the HUD
  (Utilities|FlowControl|Sequence
    (:then_0
      (bind _asbp_first_person_character (Utilities|Casting|CastToBP_FirstPersonCharacter (Game|GetPlayerCharacter 0)))
      (Utilities|IsValid _asbp_first_person_character
        (:Is%20Valid
          (if (and (== (Variables|/Game/AdvanceWeaponPack/FirstPersonContent/Blueprints/BP_FirstPersonCharacter.BP_FirstPersonCharacter_C|GetHitComponent _asbp_first_person_character) (Variables|Default|GetBox)) (Variables|Default|GetIsInRange?))
            (Utilities|IsValid _player
              (:Is%20Valid
                (Variables|/Game/AdvanceWeaponPack/Widget/PickUpHUD.PickUpHUD_C|SetName _pickuphud (Utilities|Text|ToText(Name) (.Name (Utilities|Struct|BreakInventory_Struct (Variables|Default|GetInventoryStruct)))))
                (Variables|/Game/AdvanceWeaponPack/Widget/PickUpHUD.PickUpHUD_C|SetIsInRange? _pickuphud true)
                (Widget|SetVisibility _pickuphud "Visible")
                (switch Utilities|FlowControl|Switch|SwitchonAttachmentType_Enum _attachmenttype
                  (:NewEnumerator0
                    _)
                  (:NewEnumerator1
                    _)
                  (:NewEnumerator2
                    _)
                  (:NewEnumerator3
                    _)
                  (:NewEnumerator4
                    _)
                  (:NewEnumerator5
                    _)
                  (:NewEnumerator6
                    _))
                (Appearance|SetBrushfromTexture _attachmentimage _itemimage false)
                (Widget|SetVisibility _attachmentimage "Visible")
                (Widget|SetVisibility (Variables|/Game/AdvanceWeaponPack/Widget/PickUpHUD.PickUpHUD_C|GetWeaponImage _pickuphud_2) "Hidden")))))))
    (:then_1
      (if (Variables|/Script/Engine.PlayerController|GetbShowMouseCursor (Game|GetPlayerController 0))
        (Utilities|IsValid _pickuphud
          (:Is%20Valid
            (Widget|SetVisibility _pickuphud "Collapsed")))))))

(fn ConstructionScript)