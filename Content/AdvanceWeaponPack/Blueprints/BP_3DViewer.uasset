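; 3D weapon viewer for the loadout screen that shows child-actor weapons with drag rotation and camera zoom.
; Mouse drag rotates the Scene component, and on release a timeline eases roll and pitch back to level while keeping yaw.
; Zoom timelines lerp the camera between per-category marker locations, picked from the player's LoadoutWidget selection.
; BeginPlay caches the first-person character and resets several weapons to their default materials.
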(event Custom|OnClickStart
  (params (MouseLocation :type Vector%202D%20Structure))
  ;[1 1 1] Drag & Drop Setup
  (Variables|Default|SetOnStartRotateLocation MouseLocation)
  (Variables|Default|SetRotationEnabled true))

(event Custom|OnMouseMove
  (params (MouseLocation :type Vector%202D%20Structure))
  ;[1 1 1] Drag & Drop Setup
  (if (Variables|Default|GetRotationEnabled)
    (Transformation|AddRelativeRotation (Variables|Default|GetScene) (Math|Rotator|MakeRotator (/ (.y (- MouseLocation (Variables|Default|GetOnStartRotateLocation))) -3.0) 0.0 (/ (.x (- MouseLocation (Variables|Default|GetOnStartRotateLocation))) -3.0)) false false)
    (Variables|Default|SetOnStartRotateLocation MouseLocation)))

(event Custom|3DLerp
  ;[1 1 1] Trasition of Weapon
  (CallFunction|SetStart&EndLocation)
  (bind _newtrack_0 (Timeline|LerpCamera PlayFromStart)
    (:Update
      (Transformation|SetRelativeLocation (Variables|Default|GetCamera) (Math|Vector|Lerp(Vector) (Variables|Default|GetStartLocation) (Variables|Default|GetEndLocation) _newtrack_0) false false))))

(event Custom|OnClickedEnd
  (bind _scene (Variables|Default|GetScene))
  (bind _returnvalue (Transformation|GetWorldRotation _scene))
  ;[1 1 1] Drag & Drop Setup
  (Variables|Default|SetRotationEnabled false)
  (Variables|Default|SetAlpha 0.0)
  (EventDispatchers|BindEventtoOnReleased (Game|GetPlayerController 0) (delegate Custom|CustomEvent_0))
  (bind _newtrack_0 (Timeline|RotationTImeline PlayFromStart)
    (:Update
      (bind _output_get (Variables|Default|SetAlpha _newtrack_0))
      (Transformation|SetRelativeRotation (Variables|Default|GetScene) (Math|Rotator|Lerp(Rotator) (Math|Rotator|MakeRotator (.roll _returnvalue) (.pitch _returnvalue) (.yaw _returnvalue)) (Math|Rotator|MakeRotator 0.0 0.0 (.yaw _returnvalue)) _output_get true) false false))))

(event Custom|3DLerpRev
  ;[1 1 1] Trasition of Weapon
  (bind _newtrack_0 (Timeline|LerpCameraRev PlayFromStart)
    (:Update
      (Transformation|SetRelativeLocation (Variables|Default|GetCamera) (Math|Vector|Lerp(Vector) (Variables|Default|GetEndLocation) (Variables|Default|GetStartLocation) _newtrack_0) false false))))

(event Custom|CustomEvent_0
  (params (TouchedActor :type Actor%20Object%20Reference) (ButtonReleased :type Key%20Structure))
  ;[1 1 1] Drag & Drop Setup
)

(event EventBeginPlay
  ;[1 1 1] Set Default Material Instance & Scene Location
  (bind _asbp_first_person_character (Utilities|Casting|CastToBP_FirstPersonCharacter (Game|GetPlayerCharacter 0)))
  (Variables|Default|SetPlayer _asbp_first_person_character)
  (CallFunction|SetDefaultMaterialInstance))

(fn ConstructionScript)

(fn SetDefaultMaterialInstance
  (Utilities|FlowControl|Sequence
    (:then_0
      (bind _asbp_eon_conv_smg (Utilities|Casting|CastToBP_EonConv_SMG (Variables|/Script/Engine.ChildActorComponent|GetChildActor (Variables|Default|GetEonConv_SMG))))
      (Utilities|IsValid _asbp_eon_conv_smg
        (:Is%20Valid
          (Default|SetDefaultMaterial _asbp_eon_conv_smg -4.0))))
    (:then_1
      (bind _asbp_karos_handgun (Utilities|Casting|CastToBP_Karos_Handgun (Variables|/Script/Engine.ChildActorComponent|GetChildActor (Variables|Default|GetKaros_Handgun))))
      (Utilities|IsValid _asbp_karos_handgun
        (:Is%20Valid
          (Default|SetDefaultMaterial _asbp_karos_handgun -4.0))))
    (:then_2
      (bind _asbp_ls80_assault (Utilities|Casting|CastToBP_LS80_Assault (Variables|/Script/Engine.ChildActorComponent|GetChildActor (Variables|Default|GetLS80_Assault))))
      (Utilities|IsValid _asbp_ls80_assault
        (:Is%20Valid
          (Default|SetDefaultMaterial _asbp_ls80_assault -4.0))))
    (:then_4
      (bind _asbp_roger_lr220__handgun (Utilities|Casting|CastToBP_RogerLR220__Handgun (Variables|/Script/Engine.ChildActorComponent|GetChildActor (Variables|Default|GetRogerLR220__Handgun))))
      (Utilities|IsValid _asbp_roger_lr220__handgun
        (:Is%20Valid
          (Default|SetDefaultMaterial _asbp_roger_lr220__handgun -4.0))))
    (:then_5
      (bind _asbp_double_barrel_shotgun (Utilities|Casting|CastToBP_DoubleBarrel_Shotgun (Variables|/Script/Engine.ChildActorComponent|GetChildActor (Variables|Default|GetDoubleBarrel_Shotgun))))
      (Utilities|IsValid _asbp_double_barrel_shotgun
        (:Is%20Valid
          (Default|SetDefaultMaterial _asbp_double_barrel_shotgun -4.0))))
    (:then_6
      (bind _asbp_c7_asault (Utilities|Casting|CastToBP_C7_Asault (Variables|/Script/Engine.ChildActorComponent|GetChildActor (Variables|Default|GetC7_Asault))))
      (Utilities|IsValid _asbp_c7_asault
        (:Is%20Valid
          (Default|SetDefaultMaterial _asbp_c7_asault -4.0))))))

(fn SetStart&EndLocation
  (switch int (Variables|/Game/AdvanceWeaponPack/Widget/Loadout/Loadout_Widget.Loadout_Widget_C|GetSelect%20Weapon (Variables|/Game/AdvanceWeaponPack/FirstPersonContent/Blueprints/BP_FirstPersonCharacter.BP_FirstPersonCharacter_C|GetLoadoutWidget (Variables|Default|GetPlayer)))
    (:0
      (Variables|Default|SetStartLocation (Transformation|GetWorldLocation (Variables|Default|GetHandgunInitialLocation)) :!label _label)
      (Variables|Default|SetEndLocation (Transformation|GetWorldLocation (Variables|Default|GetHandgunZoomedLocation))))
    (:1
      (goto _label))
    (:2
      (Variables|Default|SetStartLocation (Transformation|GetWorldLocation (Variables|Default|GetSMGInitialLocation)) :!label _label_2)
      (Variables|Default|SetEndLocation (Transformation|GetWorldLocation (Variables|Default|GetSMGZoomedLocation))))
    (:3
      (goto _label_2))
    (:4
      (Variables|Default|SetStartLocation (Transformation|GetWorldLocation (Variables|Default|GetAssaultInitialLocation)) :!label _label_3)
      (Variables|Default|SetEndLocation (Transformation|GetWorldLocation (Variables|Default|GetAssaultZoomedLocation))))
    (:5
      (Variables|Default|SetStartLocation (Transformation|GetWorldLocation (Variables|Default|GetShotgunInitialLocation)) :!label _label_4)
      (Variables|Default|SetEndLocation (Transformation|GetWorldLocation (Variables|Default|GetShotgunZoomedLocation))))
    (:6
      (goto _label_3))
    (:7
      (Variables|Default|SetStartLocation (Transformation|GetWorldLocation (Variables|Default|GetSpecialInitialLocation)) :!label _label_5)
      (Variables|Default|SetEndLocation (Transformation|GetWorldLocation (Variables|Default|GetSpecialZoomedLocation))))
    (:8
      (goto _label_4))
    (:9
      (goto _label_3))
    (:10
      (goto _label_5))
    (:11
      (goto _label_5))
    (:12
      (goto _label_5))))