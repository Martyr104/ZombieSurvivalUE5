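; Laser actor, named for the 9mm weapon, that draws a beam and end decal while IsLaserOn is set, hiding both otherwise.
; StartLaser runs on construction and every Tick, line-tracing forward on Visibility to set the particle beam's endpoint and decal distance.
; It disables the Box's collision before tracing, then scales and offsets it by beam length and re-enables it.
; BeginPlay caches the first-person player character, unused in these graphs.
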(event EventBeginPlay
  (bind _asbp_first_person_character (Utilities|Casting|CastToBP_FirstPersonCharacter (Game|GetPlayerCharacter 0)))
  (Variables|Default|SetPlayer _asbp_first_person_character))

(event EventTick
  (params (DeltaSeconds :type Float%20%28single-precision%29))
  (CallFunction|StartLaser))

(fn ConstructionScript
  (CallFunction|StartLaser))

(fn ScaleTriggerBox
  (params (EndPoint :type Vector))
  (bind _laserstartpoint (Variables|Default|GetLaserStartPoint))
  (bind _box (Variables|Default|GetBox))
  (bind _returnvalue (Transformation|GetWorldLocation _laserstartpoint))
  (bind _returnvalue_2 (- EndPoint _returnvalue))
  (bind _returnvalue_3 (Math|Vector|VectorLength _returnvalue_2))
  (bind _returnvalue_4 (/ _returnvalue_3 2.0))
  (bind _returnvalue_5 (Math|Vector|MakeVector _returnvalue_4 0.0 0.0))
  (Transformation|SetRelativeScale3D _box _returnvalue_5)
  (Transformation|SetRelativeLocation _box (+ (Variables|/Script/Engine.SceneComponent|GetRelativeLocation _box) _returnvalue_5) false false))

(fn StartLaser
  (bind _laserstartpoint (Variables|Default|GetLaserStartPoint))
  (bind _returnvalue (Transformation|GetWorldLocation _laserstartpoint))
  (Collision|SetCollisionEnabled (Variables|Default|GetBox) "NoCollision")
  (if (Variables|Default|GetIsLaserOn?)
    (Rendering|SetVisibility (Variables|Default|GetLaser_ParticleSystem) true false)
    (bind _output_get (Variables|Default|SetEndBeamPoint (+ _returnvalue (* (Math|Vector|GetForwardVector _laserstartpoint) 500000))))
    (bind (_outhit _returnvalue_2) (Collision|LineTraceByChannel _returnvalue _output_get "TraceTypeQuery1" false 0 "None"))
    (if _returnvalue_2
      (bind _output_get_2 (Variables|Default|SetEndBeamPoint (.Location (Collision|BreakHitResult _outhit)))))
    (Class|ParticleSystemComponent|SetBeamEndPoint (Variables|Default|GetLaser_ParticleSystem) 0 _output_get_2)
    (CallFunction|ScaleTriggerBox (Variables|Default|GetEndBeamPoint))
    (Collision|SetCollisionEnabled (Variables|Default|GetBox) "QueryAndPhysics")
    (Transformation|SetRelativeLocation (Variables|Default|GetDecal) (Math|Vector|MakeVector (Math|Vector|VectorLength (- (.Location (Collision|BreakHitResult _outhit)) (Transformation|GetSocketLocation (Variables|Default|GetLaserStartPoint) "None"))) 0.0 0.0) false true)
    (else
      (Rendering|SetVisibility (Variables|Default|GetLaser_ParticleSystem) false false))))