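; BP_PlayerController is the player controller that creates the HUD on begin play and toggles the in-game menu from an input action.
; OpenWidget either spawns and focuses a widget in UI-only input mode or removes the open one, without restoring game input.
; RemoveWidget separately restores game-only input, hides the cursor and re-enables character input, but leaves the open flag untouched.
; The logic to disable character input and stop movement is disconnected.
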(event EventBeginPlay
  (bind _returnvalue (UserInterface|CreateWidget "/Game/Project/UI/WB_HUD.WB_HUD_C" self))
  (UserInterface|Viewport|AddtoViewport _returnvalue 0)
  (Variables|Default|SetbShowMouseCursor false)
  (bind _asbp_player_character (Utilities|Casting|CastToBP_PlayerCharacter (Pawn|GetControlledPawn)))
  (Variables|Default|SetAs%20BP%20Player%20Character _asbp_player_character))

(event Input|ActionEvents|InputActionInGameMenu
  (params (Key :type Key%20Structure :default "None"))
  (:Pressed
    (CallFunction|OpenWidget "/Game/Project/UI/WB_InGameMenu.WB_InGameMenu_C")))

(fn ConstructionScript)

(fn RemoveWidget
  (params (Widget%20to%20Remove :type User%20Widget%20Object%20Reference))
  (Widget|RemovefromParent Widget%20to%20Remove)
  (Input|SetInputModeGameOnly self)
  (Variables|Default|SetbShowMouseCursor false)
  (Input|EnableInput (Variables|Default|GetAs%20BP%20Player%20Character) self))

(fn OpenWidget
  (params (Class :type User%20Widget%20Class%20Reference))
  (bind _self self)
  (if (Variables|Default|GetIsWidgetOpen)
    (Variables|Default|SetIsWidgetOpen false)
    (Widget|RemovefromParent (Variables|Default|GetCurrentFocusedWidget))
    (else
      (Variables|Default|SetIsWidgetOpen true)
      (bind _returnvalue (UserInterface|CreateWidget Class _self))
      (UserInterface|Viewport|AddtoViewport _returnvalue 0)
      (Variables|Default|SetCurrentFocusedWidget _returnvalue)
      (Input|SetInputModeUIOnly _self _returnvalue "DoNotLock"))))