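; BP_PlayerState tracks the player's health and pushes it to the HUD and health bar widgets.
; Health starts at maximum in the construction script, and BeginPlay caches the player character.
; UpdateHealth effectively adds DamageValue to current health, without clamping, then refreshes both widgets with the health percentage and prints a debug message.
; The widget references are not assigned within this Blueprint.
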(event EventBeginPlay
  (bind _asbp_player_character (Utilities|Casting|CastToBP_PlayerCharacter (Game|Player|GetPlayerPawn 0)))
  (Variables|Default|SetAs%20BP%20Player%20Character _asbp_player_character))

(fn ConstructionScript
  (Variables|Default|SetPlayerCurrentHealth (Variables|Default|GetPlayerMaxHealth)))

(fn UpdateHealth
  (params (Damage%20Value :type Float%20%28single-precision%29))
  (Variables|Default|SetPlayerCurrentHealth (- (Variables|Default|GetPlayerCurrentHealth) (* Damage%20Value -1.0)))
  (CallFunction|UpdateHealthWidgets))

(fn UpdateHealthWidgets
  (bind _playercurrenthealth (Variables|Default|GetPlayerCurrentHealth))
  (bind _playermaxhealth (Variables|Default|GetPlayerMaxHealth))
  (bind _output (Utilities|MakePercentage _playercurrenthealth _playermaxhealth))
  (Variables|/Game/Project/UI/WB_HUD.WB_HUD_C|SetHealthBarVar (Variables|Default|GetWB%20HUD%20Ref) _output)
  (Variables|/Game/Project/UI/WB_HealthBar.WB_HealthBar_C|SetHealthBarVar (Variables|Default|GetWB%20HealthBar%20Ref) _output)
  (Development|PrintString (Utilities|String|Append "Setting health widget to " (Utilities|String|ToString(Float) _output))))